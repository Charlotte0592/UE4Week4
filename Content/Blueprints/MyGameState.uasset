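; Game state Blueprint that runs the match countdown and triggers the game over screen.
; Tick feeds a one-second looping Delay that decrements RemainTime.
; At zero or below, it creates the GameOver widget, adds it to the viewport and shows player 0's mouse cursor; Tick keeps re-entering the Delay, so this branch can repeat.
; The OnRep functions for GameStartTimer and RandomTimerValue1 are empty.
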(event EventTick
  (params (DeltaSeconds :type Float%20%28single-precision%29))
  ;[1 1 1] Countdown
  (Utilities|FlowControl|Delay 1.0 :!label _label)
  (bind _output_get (Variables|Default|SetRemainTime (- (Variables|Default|GetRemainTime) 1)))
  (if (<= _output_get 0)
    ;[1 1 1] Show the Game Over Info
    (bind _returnvalue (UserInterface|CreateWidget "/Game/Blueprints/Widgets/GameOver.GameOver_C"))
    (bind _output_get_2 (Variables|Default|SetGameOverWidget _returnvalue))
    (UserInterface|Viewport|AddtoViewport _output_get_2 0)
    (Variables|/Script/Engine.PlayerController|SetbShowMouseCursor (Game|GetPlayerController 0) true)
    (else
      (goto _label))))

(fn ConstructionScript)

(fn OnRepGameStartTimer)

(fn OnRepRandomTimerValue1)